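; Player controller for the main menu that creates and shows the WB_MainMenu widget.
; On BeginPlay it adds the widget to the viewport, shows the mouse cursor and sets Game and UI input focused on the menu.
; The first press of any key calls the widget's FindGameTrigger, with a DoOnce gate ignoring later presses.
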(event EventBeginPlay
  (bind _returnvalue (UserInterface|CreateWidget "/Game/UI/WB_MainMenu.WB_MainMenu_C"))
  (bind _output_get (Variables|Default|SetMainMenu _returnvalue))
  (UserInterface|Viewport|AddtoViewport _output_get 0)
  (Variables|Default|SetbShowMouseCursor true)
  (Input|SetInputModeGameandUI self (Variables|Default|GetMainMenu) "DoNotLock" true))

(event Input|KeyboardEvents|AnyKey
  (params (Key :type Key%20Structure))
  (:Pressed
    (Utilities|FlowControl|DoOnce false
      (:Completed
        (Default|FindGameTrigger (Variables|Default|GetMainMenu))))))

(fn ConstructionScript)