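; BP_Human is a player-controlled pawn that moves along world axes through the MoveForward and MoveRight input axes.
; Forward input, gated by CanMoveForward, moves it along X, clamps its location between fixed bounds and prints a debug check of X.
; The same event sets IsMovingForward while X is strictly inside those bounds, which blocks sideways Y movement until the pawn is at either end.
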(event Input|AxisEvents|InputAxisMoveRight
  (params (AxisValue :type Float%20%28single-precision%29))
  (if (and (!= AxisValue 0.0) (not (Variables|Default|GetisMovingForward)))
    (Pawn|Input|AddMovementInput (Math|Vector|MakeVector 0.0 (* AxisValue (Variables|Default|GetmoveSpeed)) 0.0) 1.0 false)))

(event Input|AxisEvents|InputAxisMoveForward
  (params (AxisValue :type Float%20%28single-precision%29))
  (bind _returnvalue (Transformation|GetActorLocation))
  (bind _returnvalue_2 (> (.x _returnvalue) 0.0))
  (if (Variables|Default|GetcanMoveForward)
    (Pawn|Input|AddMovementInput (Math|Vector|MakeVector (* AxisValue (Variables|Default|GetmoveSpeed)) 0.0 0.0) 1.0 false)
    (Development|PrintString (Utilities|String|ToString(Boolean) _returnvalue_2))
    (Variables|Default|SetisMovingForward (and _returnvalue_2 (< (.x _returnvalue) 5e+02)))
    (Transformation|SetActorLocation (Math|Vector|MakeVector (Math|Float|Clamp(Float) (.x _returnvalue) 0.0 5e+02) (.y _returnvalue) (.z _returnvalue)) false false)))

(fn ConstructionScript)